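; Stormtrooper character Blueprint with a health value and an on-screen health bar.
; On BeginPlay it creates the HealthBarHUD widget, adds it to the viewport and sets the walk speed from the Velocidad field of Datos.
; Hard-wired F and V keys lower and raise CurrentHealth by one, with no clamping or explicit HUD update in the graph.
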(event `Key|F`
  (params (Key :type "Key Structure"))
  (:`Pressed`
    (set `self.CurrentHealth` (- (`self.CurrentHealth`) 1.0))))

(event `Key|V`
  (params (Key :type "Key Structure"))
  (:`Pressed`
    (set `self.CurrentHealth` (+ (`self.CurrentHealth`) 1.0))))

(event `self.ReceiveBeginPlay`
  (bind (_datos_nombre _datos_velocidad) (break `/Game/Blueprint/datos` (`self.Datos`)))
  (bind _returnvalue (`|CreateWidget` "/Game/HealthBarHUD.HealthBarHUD_C"))
  (bind _output_get (set `self.Healthbarreference` _returnvalue))
  (`UserWidget.AddToViewport` _output_get 0)
  (set `CharacterMovementComponent.MaxWalkSpeed` _datos_velocidad (`self.CharacterMovement`)))

(fn `UserConstructionScript`
  (`parent.UserConstructionScript`))