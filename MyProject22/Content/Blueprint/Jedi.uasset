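; Jedi character Blueprint with health and shield values, each shown through its own HUD widget.
; On BeginPlay it creates and stores the health and shield bar widgets, adds them to the viewport, and sets max walk speed from the Velocidad field of Datos.
; Hard-wired keys F/V lower and raise health and G/T do the same for shield, in single-point steps without clamping.
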(event `Key|F`
  (params (Key :type "Key Structure"))
  (:`Pressed`
    (set `self.CurrentHealth` (- (`self.CurrentHealth`) 1.0))))

(event `Key|V`
  (params (Key :type "Key Structure"))
  (:`Pressed`
    (set `self.CurrentHealth` (+ (`self.CurrentHealth`) 1.0))))

(event `Key|G`
  (params (Key :type "Key Structure"))
  (:`Pressed`
    (set `self.CurrentShield` (- (`self.CurrentShield`) 1.0))))

(event `self.ReceiveBeginPlay`
  (bind (_datos_nombre _datos_velocidad) (break `/Game/Blueprint/datos` (`self.Datos`)))
  (`|ExecutionSequence`
    (:`then_0`
      (bind _returnvalue (`|CreateWidget` "/Game/HealthBarHUD.HealthBarHUD_C"))
      (bind _output_get (set `self.Healthbarreference` _returnvalue))
      (`UserWidget.AddToViewport` _output_get 0)
      (set `CharacterMovementComponent.MaxWalkSpeed` _datos_velocidad (`self.CharacterMovement`)))
    (:`then_1`
      (bind _returnvalue_2 (`|CreateWidget` "/Game/ShieldBarHUD.ShieldBarHUD_C"))
      (bind _output_get_2 (set `self.Shieldbarreference` _returnvalue_2))
      (`UserWidget.AddToViewport` _output_get_2 0))))

(event `Key|T`
  (params (Key :type "Key Structure"))
  (:`Pressed`
    (set `self.CurrentShield` (+ (`self.CurrentShield`) 1.0))))

(fn `UserConstructionScript`
  (`parent.UserConstructionScript`))